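; MainPlayerGameMode is a game mode Blueprint that links the first player's controller to its character when play begins.
; On BeginPlay it casts player 0's pawn to MainPlayerCharacter, stopping if that fails.
; It then copies the character's first-person camera, Mesh2P and gun onto MainPlayerController.
; The gun reference comes from the Gun child actor component, cast to WeaponBaseBp.
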(event EventBeginPlay
  (bind _returnvalue (Game|GetPlayerController 0))
  (bind _asmain_player_controller (Utilities|Casting|CastToMainPlayerController _returnvalue))
  (bind _asmain_player_character (Utilities|Casting|CastToMainPlayerCharacter (Game|GetPlayerCharacter 0)))
  (Variables|/Game/Blueprints/CharacterBp/MainPlayerController.MainPlayerController_C|SetFirstPersonCamera _asmain_player_controller (Variables|/Game/Blueprints/CharacterBp/MainPlayerCharacter.MainPlayerCharacter_C|GetFirstPersonCamera _asmain_player_character))
  (Variables|/Game/Blueprints/CharacterBp/MainPlayerController.MainPlayerController_C|SetGun _asmain_player_controller (.AsWeapon%20Base%20Bp (Utilities|Casting|CastToWeaponBaseBp (Variables|/Script/Engine.ChildActorComponent|GetChildActor (Variables|/Game/Blueprints/CharacterBp/MainPlayerCharacter.MainPlayerCharacter_C|GetGun _asmain_player_character)))))
  (Variables|/Game/Blueprints/CharacterBp/MainPlayerController.MainPlayerController_C|SetMesh2P _asmain_player_controller (Variables|/Game/Blueprints/CharacterBp/MainPlayerCharacter.MainPlayerCharacter_C|GetMesh2P _asmain_player_character)))

(fn ConstructionScript)