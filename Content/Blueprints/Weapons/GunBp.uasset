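; Gun weapon Blueprint that fires a projectile when its child attack event runs.
; The construction script attaches the Muzzle component to the Muzzle socket on Gun.
; The attack spawns ProjectileClass at ProjectileSpawnTransform, adjusting for collisions but always spawning, then prints the muzzle's scaled forward vector as debug output.
; An impulse push on the spawned PlayerProjectileBp's sphere is left disconnected and never runs.
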(event EventBeginPlay
  (|CallParentFunction) ; This node is disabled and will not be called.\nDrag off pins to build functionality.
)

(event Collision|EventActorBeginOverlap
  (params (OtherActor :type Actor%20Object%20Reference))
  (|CallParentFunction OtherActor) ; This node is disabled and will not be called.\nDrag off pins to build functionality.
)

(event EventTick
  (params (DeltaSeconds :type Float%20%28single-precision%29))
  (|CallParentFunction DeltaSeconds) ; This node is disabled and will not be called.\nDrag off pins to build functionality.
)

(event EventEventChildAttack
  (bind _returnvalue (Game|SpawnActorfromClass (Variables|Default|GetProjectileClass) (Variables|Default|GetProjectileSpawnTransform) "AdjustIfPossibleButAlwaysSpawn" 0 0))
  (Development|PrintString (Utilities|String|ToString(Vector) (* (Math|Vector|GetForwardVector (Transformation|GetWorldRotation (Variables|Default|GetMuzzle))) 1e+02))))

(fn ConstructionScript
  (|CallParentFunction)
  (Transformation|AttachComponentToComponent (Variables|Default|GetMuzzle) (Variables|Default|GetGun) "Muzzle" "KeepRelative" "KeepRelative" "KeepRelative" true))